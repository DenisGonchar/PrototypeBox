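; BP_projectileVFXSpawner is an actor meant to repeatedly spawn projectile VFX at its location, but its logic is disconnected.
; BeginPlay and SpawnProjectileVFX are empty; the looping timer and spawn chain never run.
; The orphaned chain spawns an actor, then sets its muzzle, projectile and impact effects, X-axis velocity and destroy delay.
; The spawned-projectile reference reads None, suggesting a broken link.
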(event Custom|SpawnProjectileVFX)

(event EventBeginPlay)

(fn ConstructionScript)