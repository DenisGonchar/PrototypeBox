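; Master projectile Blueprint for VFX-driven projectiles, spawning a muzzle effect at its location just after BeginPlay.
; When its box collision overlaps a BlockingVolume, it stops movement and spawns the hit impact effect.
; It also sets the ShouldKillMainSlash parameter on its VFX component to end the main slash, then destroys itself after a configurable delay.
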(event OnComponentBeginOverlap(ProjectileBoxCollision)
  (params (OverlappedComponent :type Primitive%20Component%20Object%20Reference) (OtherActor :type Actor%20Object%20Reference) (OtherComp :type Primitive%20Component%20Object%20Reference) (OtherBodyIndex :type Integer) (bFromSweep :type Boolean) (SweepResult :type Hit%20Result%20Structure%20%28by%20ref%29))
  (Utilities|Casting|CastToBlockingVolume OtherActor)
  (Components|Movement|StopMovementImmediately (Variables|Default|GetProjectileVFXMovementComp))
  (Class|NiagaraComponent|SetVariableBool (Variables|Default|GetProjectileVFX_Compponent) "ShouldKillMainSlash" true)
  (CallFunction|SpawnFVX (Variables|Default|GetHitImpactVFX))
  (Utilities|FlowControl|Delay (Variables|Default|GetProjectileDestroyDelay))
  (Actor|DestroyActor))

(event EventBeginPlay
  (Utilities|FlowControl|Delay 0.01)
  (CallFunction|SpawnFVX (Variables|Default|GetMuzzleVFX)))

(fn ConstructionScript)

(fn SpawnFVX
  (params (VFXToSpawn :type Niagara%20System%20Object%20Reference))
  (Utilities|IsValid VFXToSpawn
    (:Is%20Valid
      (Niagara|SpawnSystematLocation VFXToSpawn (Transformation|GetActorLocation)))))