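; Game instance that acts as the hub for the game's menus and persistent save data.
; Events lazily create and cache widgets for main, pause, win, options, level, achievement and save screens, with some also setting pause, cursor and input mode.
; Save functions read and write PSSaveGame level records, replacing entries with matching level names.
; Separate BP_SaveGame slots store sound volumes and Restart/Reset input bindings.
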(event Custom|ShowMenuAcheve
  ;[1 1 1] Вызрв меню ачивок  в меню
  (Utilities|IsValid (Variables|Default|GetAchevMenuWidget)
    (:Is%20Valid
      _)
    (:Is%20Not%20Valid
      (bind _returnvalue (UserInterface|CreateWidget "/Game/Project/Widget/Menu/Achevements/BPW_AchivMenu.BPW_AchivMenu_C" (Game|GetPlayerController 0)))
      (bind _output_get (Variables|Default|SetAchevMenuWidget _returnvalue))))
  (UserInterface|Viewport|AddtoViewport _output_get 0))

(event Custom|RemovSaveSlot
  ;[1 1 1] Comment
  (Widget|RemovefromParent (Variables|Default|GetSaveMenuWidget)))

(event Custom|Save
  (params (NewItem :type Level%20Data%20Structure%20%28by%20ref%29))
  (CallFunction|SaveLvl NewItem))

(event Custom|ShowSaveSlot
  (Utilities|IsValid (Variables|Default|GetSaveSlotWidget)
    (:Is%20Valid
      _)
    (:Is%20Not%20Valid
      (bind _returnvalue (UserInterface|CreateWidget "/Game/Project/Widget/Menu/SaveSlot/BPW_SaveSlot.BPW_SaveSlot_C" (Game|GetPlayerController 0)))
      (bind _output_get (Variables|Default|SetSaveSlotWidget _returnvalue))))
  (UserInterface|Viewport|AddtoViewport _output_get 0))

(event Custom|DeletComixs
  ;[1 1 1] Comment
  (Widget|RemovefromParent (Variables|Default|GetComicsWidget))
  (CallFunction|ShowSaveMenu))

(event Custom|ShowAcepptBox
  (params (SaveName :type String))
  ;[1 1 1] Comment
  (Utilities|IsValid (Variables|Default|GetAcepptBoxWidget)
    (:Is%20Valid
      _)
    (:Is%20Not%20Valid
      (bind _returnvalue (UserInterface|CreateWidget "/Game/Project/Widget/Menu/SaveSlot/BPW_AcceptBox.BPW_AcceptBox_C" (Game|GetPlayerController 0) SaveName))
      (bind _output_get (Variables|Default|SetAcepptBoxWidget _returnvalue))))
  (UserInterface|Viewport|AddtoViewport _output_get 0))

(event Custom|ShowY_NLevel
  ;[1 1 1] Вызов меню да нет
  (Utilities|IsValid (Variables|Default|GetY_NLevelWidget)
    (:Is%20Valid
      _)
    (:Is%20Not%20Valid
      (bind _returnvalue (UserInterface|CreateWidget "/Game/Project/Widget/Menu/Pause/BPW_Y_NLevel.BPW_Y_NLevel_C" (Game|GetPlayerController 0)))
      (bind _output_get (Variables|Default|SetY_NLevelWidget _returnvalue))))
  (UserInterface|Viewport|AddtoViewport _output_get 0))

(event Custom|PauseMenuToMainMenuDecline
  ;[1 1 1] Menu pause to main menu
  (Widget|RemovefromParent (Variables|Widget|GetPauseMenuToMainManuWidget))
  (UserInterface|Viewport|AddtoViewport (Variables|Widget|GetPauseManuWidget) 0))

(event Custom|DeletSaveSlot
  ;[1 1 1] Comment
  (Widget|RemovefromParent (Variables|Default|GetSaveMenuWidget)))

(event Custom|ShowSaveMenu
  ;[1 1 1] Вызрв меню сохранения
  (Utilities|IsValid (Variables|Default|GetSaveMenuWidget)
    (:Is%20Valid
      _)
    (:Is%20Not%20Valid
      (bind _returnvalue (UserInterface|CreateWidget "/Game/Project/Widget/Menu/SaveSlot/WBP_SaveMenu.WBP_SaveMenu_C" (Game|GetPlayerController 0)))
      (bind _output_get (Variables|Default|SetSaveMenuWidget _returnvalue))))
  (UserInterface|Viewport|AddtoViewport _output_get 0))

(event Custom|ShowSettinginPause
  ;[1 1 1] Вызрв меню ачивок
  (Utilities|IsValid (Variables|Default|GetOptionsPauseWidget)
    (:Is%20Valid
      _)
    (:Is%20Not%20Valid
      (bind _returnvalue (UserInterface|CreateWidget "/Game/Project/Widget/Menu/Setting/BPW_Option_MenuPause.BPW_Option_MenuPause_C" (Game|GetPlayerController 0)))
      (bind _output_get (Variables|Default|SetOptionsPauseWidget _returnvalue))))
  (UserInterface|Viewport|AddtoViewport _output_get 0))

(event Custom|ShowAcivePause
  ;[1 1 1] Вызрв меню ачивок в паузе
  (Utilities|IsValid (Variables|Widget|GetAcivePauseWidget)
    (:Is%20Valid
      _)
    (:Is%20Not%20Valid
      (bind _returnvalue (UserInterface|CreateWidget "/Game/Project/Widget/Menu/Achevements/BPW_AchivPause.BPW_AchivPause_C" (Game|GetPlayerController 0)))
      (bind _output_get (Variables|Widget|SetAcivePauseWidget _returnvalue))))
  (UserInterface|Viewport|AddtoViewport _output_get 0))

(event Custom|ShowCredits
  ;[1 1 1] Options menu
  (Utilities|IsValid (Variables|Widget|GetCreditsWidget)
    (:Is%20Valid
      _)
    (:Is%20Not%20Valid
      (bind _returnvalue (UserInterface|CreateWidget "/Game/Project/Widget/Menu/Credits/BPW_Credits.BPW_Credits_C" (Game|GetPlayerController 0)))
      (bind _output_get (Variables|Widget|SetCreditsWidget _returnvalue))))
  (UserInterface|Viewport|AddtoViewport _output_get 0))

(event Custom|PauseMenuToMainMenu
  ;[1 1 1] Menu pause to main menu
  (Utilities|IsValid (Variables|Widget|GetPauseMenuToMainManuWidget)
    (:Is%20Valid
      _)
    (:Is%20Not%20Valid
      (bind _returnvalue (UserInterface|CreateWidget "/Game/Project/Widget/Menu/Pause/BPW_Pause_Menu_To_Main_Menu.BPW_Pause_Menu_To_Main_Menu_C" (Game|GetPlayerController 0)))
      (Variables|Widget|SetPauseMenuToMainManuWidget _returnvalue)))
  (UserInterface|Viewport|AddtoViewport (Variables|Widget|GetPauseMenuToMainManuWidget) 0))

(event Custom|ShowWin
  (bind _returnvalue (Game|GetPlayerController 0))
  ;[1 1 1] Win level
  (Utilities|IsValid (Variables|Widget|GetWinLevelWidget)
    (:Is%20Valid
      _)
    (:Is%20Not%20Valid
      (bind _returnvalue_2 (UserInterface|CreateWidget "/Game/Project/Widget/BP/BPW_Win_Level.BPW_Win_Level_C" _returnvalue))
      (Variables|Widget|SetWinLevelWidget _returnvalue_2)))
  (UserInterface|Viewport|AddtoViewport (Variables|Widget|GetWinLevelWidget) 0)
  (Variables|/Script/Engine.PlayerController|SetbShowMouseCursor _returnvalue true)
  (Input|SetInputModeUIOnly _returnvalue (Variables|Widget|GetWinLevelWidget) "LockInFullscreen")
  (Game|SetGamePaused true))

(event Custom|PauseMenuResume
  (bind _returnvalue (Game|GetPlayerController 0))
  ;[1 1 1] Pause menu resume
  (Widget|RemovefromParent (Variables|Widget|GetPauseManuWidget))
  (Game|SetGamePaused false)
  (Variables|/Script/Engine.PlayerController|SetbShowMouseCursor _returnvalue false)
  (Input|SetInputModeGameOnly _returnvalue))

(event Custom|OpenLevelName
  (params (Map :type Name))
  ;[1 1 1] Open Level
  (Game|OpenLevel(byName) Map)
  (Input|SetInputModeGameOnly (Game|GetPlayerController 0)))

(event Custom|ShowMainMenu
  (bind _returnvalue (Game|GetPlayerController 0))
  ;[1 1 1] Start main menu
  (Utilities|IsValid (Variables|Widget|GetMainMenuWidget)
    (:Is%20Valid
      _)
    (:Is%20Not%20Valid
      (bind _returnvalue_2 (UserInterface|CreateWidget "/Game/Project/Widget/Menu/BPW_Main_Menu.BPW_Main_Menu_C" _returnvalue))
      (Variables|Widget|SetMainMenuWidget _returnvalue_2)))
  (UserInterface|Viewport|AddtoViewport (Variables|Widget|GetMainMenuWidget) 0)
  (Variables|/Script/Engine.PlayerController|SetbShowMouseCursor _returnvalue true)
  (Input|SetInputModeUIOnly _returnvalue (Variables|Widget|GetMainMenuWidget) "LockInFullscreen"))

(event Custom|ShowLevelsManu
  ;[1 1 1] Open levels menu
  (Utilities|IsValid (Variables|Widget|GetLevelMenuWidget)
    (:Is%20Valid
      _)
    (:Is%20Not%20Valid
      (bind _returnvalue (UserInterface|CreateWidget "/Game/Project/Widget/Menu/Levels/BPW_LevIsMenu.BPW_LevIsMenu_C" (Game|GetPlayerController 0)))
      (bind _output_get (Variables|Widget|SetLevelMenuWidget _returnvalue))))
  (UserInterface|Viewport|AddtoViewport _output_get 0))

(event Custom|ShowPauseMenu
  (bind _returnvalue (Game|GetPlayerController 0))
  ;[1 1 1] Pause menu
  (Utilities|IsValid (Variables|Widget|GetPauseManuWidget)
    (:Is%20Valid
      _)
    (:Is%20Not%20Valid
      (bind _returnvalue_2 (UserInterface|CreateWidget "/Game/Project/Widget/Menu/Pause/BPW_PauseMenu.BPW_PauseMenu_C" _returnvalue))
      (Variables|Widget|SetPauseManuWidget _returnvalue_2)))
  (UserInterface|Viewport|AddtoViewport (Variables|Widget|GetPauseManuWidget) 0)
  (Variables|/Script/Engine.PlayerController|SetbShowMouseCursor _returnvalue true)
  (Input|SetInputModeUIOnly _returnvalue (Variables|Widget|GetPauseManuWidget) "LockInFullscreen")
  (Game|SetGamePaused true))

(event Custom|ShowComics
  ;[1 1 1] Вызов виджета комикса
  (Utilities|IsValid (Variables|Default|GetComicsWidget)
    (:Is%20Valid
      _)
    (:Is%20Not%20Valid
      (bind _returnvalue (UserInterface|CreateWidget "/Game/Project/Widget/Menu/Comics/BPW_Comiks.BPW_Comiks_C" (Game|GetPlayerController 0)))
      (bind _output_get (Variables|Default|SetComicsWidget _returnvalue))))
  (UserInterface|Viewport|AddtoViewport _output_get 0))

(event Custom|PauseMenuToMainMenuAccept
  ;[1 1 1] Menu pause to main menu
  (Game|OpenLevel(byName) "Main_Menu"))

(event Custom|RemovMainMenu
  ;[1 1 1] Comment
  (Widget|RemovefromParent (Variables|Widget|GetMainMenuWidget)))

(event Custom|ShowOptionsMenu
  ;[1 1 1] Options menu
  (Utilities|IsValid (Variables|Widget|GetOptionsMenuWidget)
    (:Is%20Valid
      _)
    (:Is%20Not%20Valid
      (bind _returnvalue (UserInterface|CreateWidget "/Game/Project/Widget/Menu/Setting/BPW_Option_Menu.BPW_Option_Menu_C" (Game|GetPlayerController 0)))
      (Variables|Widget|SetOptionsMenuWidget _returnvalue)))
  (UserInterface|Viewport|AddtoViewport (Variables|Widget|GetOptionsMenuWidget) 0))

(event Custom|seve%20instanse
  (bind _returnvalue (SaveGame|DoesSaveGameExist "Volum"))
  (if _returnvalue
    (bind _returnvalue_2 (SaveGame|LoadGamefromSlot "Volum"))
    (bind _output_get (Variables|Default|SetSaveSlotRef _returnvalue_2))
    (Utilities|Casting|CastToBP_SaveGame _output_get)
    (else
      (bind _returnvalue_3 (SaveGame|CreateSaveGameObject "/Game/Project/GameMode/BP_SaveGame.BP_SaveGame_C"))
      (Variables|Default|SetSaveSlotRef _returnvalue_3))))

(event Custom|Remove%20Setting
  (Widget|RemovefromParent (Variables|Widget|GetOptionsMenuWidget)))

(event Custom|Show%20LevelPause
  ;[1 1 1] Open levels menu
  (Widget|RemovefromParent (Variables|Widget|GetPauseManuWidget))
  (Utilities|IsValid (Variables|Default|GetLevelPauseWidget)
    (:Is%20Valid
      _)
    (:Is%20Not%20Valid
      (bind _returnvalue (UserInterface|CreateWidget "/Game/Project/Widget/Menu/Levels/BPW_LevIsPause.BPW_LevIsPause_C" (Game|GetPlayerController 0)))
      (bind _output_get (Variables|Default|SetLevelPauseWidget _returnvalue))))
  (UserInterface|Viewport|AddtoViewport _output_get 0))

(fn LoadPerLevel
  (params (LevelName :type String))
  (bind _levelssaveslot (Variables|Default|GetlevelsSaveSlot))
  (bind _returnvalue (SaveGame|DoesSaveGameExist _levelssaveslot))
  (if _returnvalue
    (bind _returnvalue_2 (SaveGame|LoadGamefromSlot _levelssaveslot))
    (bind _aspssave_game (Utilities|Casting|CastToPSSaveGame _returnvalue_2))
    (if (> (Utilities|Array|Length (Variables|/Script/PrototypeStrategy.PSSaveGame|Getlevels _aspssave_game)) 0)
      (for _array_element (Variables|/Script/PrototypeStrategy.PSSaveGame|Getlevels _aspssave_game)
        (if (Utilities|Enum|Equal(Enum) LevelName (.levelName (Utilities|Struct|BreakLevelData _array_element)))
          (return _array_element)))
      (else
        (Development|PrintString "Hello")))))

(fn Load
  (bind _levelssaveslot (Variables|Default|GetlevelsSaveSlot))
  (bind _returnvalue (SaveGame|DoesSaveGameExist _levelssaveslot))
  (if _returnvalue
    (bind _returnvalue_2 (SaveGame|LoadGamefromSlot _levelssaveslot))
    (bind _aspssave_game (Utilities|Casting|CastToPSSaveGame _returnvalue_2))
    (return (Variables|/Script/PrototypeStrategy.PSSaveGame|Getlevels _aspssave_game))))

(fn SaveLvl
  (params (LevelData :type Level%20Data%20Structure%20%28by%20ref%29))
  (bind _levelssaveslot (Variables|Default|GetlevelsSaveSlot))
  (bind _levelssaveslot_2 (Variables|Default|GetlevelsSaveSlot))
  (if (Utilities|Enum|NotEqual(Enum) (.levelName (Utilities|Struct|BreakLevelData LevelData)) "")
    (bind _levels (CallFunction|Load))
    (bind (_array_element _array_index) (Utilities|Array|ForEachLoopwithBreak _levels :!label _label)
      (:LoopBody
        (if (Utilities|Enum|Equal(Enum) (.levelName (Utilities|Struct|BreakLevelData _array_element)) (.levelName (Utilities|Struct|BreakLevelData LevelData)))
          (LocalVariables|SetIsDuplicate? true)
          (LocalVariables|SetDuplicateLevelIndex _array_index)
          (Development|PrintString "Finded")
          (goto _label Break)
          (else
            (LocalVariables|SetIsDuplicate? false))))
      (:Completed
        (LocalVariables|SetLevelToSave LevelData)
        (if (LocalVariables|GetIsDuplicate?)
          (bind _returnvalue (SaveGame|DoesSaveGameExist (Variables|Default|GetlevelsSaveSlot)))
          (if _returnvalue
            (bind _returnvalue_2 (SaveGame|LoadGamefromSlot _levelssaveslot))
            (bind _aspssave_game (Utilities|Casting|CastToPSSaveGame _returnvalue_2))
            (Utilities|Array|SetArrayElem (Variables|/Script/PrototypeStrategy.PSSaveGame|Getlevels _aspssave_game) (LocalVariables|GetDuplicateLevelIndex) (LocalVariables|GetLevelToSave))
            (bind _returnvalue_3 (SaveGame|SaveGametoSlot _returnvalue_2 _levelssaveslot))
            (if _returnvalue_3
              (Development|PrintString "Resaved" :!label _label_2))
            (else
              (bind _returnvalue_4 (SaveGame|CreateSaveGameObject "/Script/PrototypeStrategy.PSSaveGame"))
              (Utilities|Array|SetArrayElem (Variables|/Script/PrototypeStrategy.PSSaveGame|Getlevels _returnvalue_4) (LocalVariables|GetDuplicateLevelIndex) (LocalVariables|GetLevelToSave))
              (bind _returnvalue_5 (SaveGame|SaveGametoSlot _returnvalue_4 _levelssaveslot))
              (if _returnvalue_5
                (goto _label_2))))
          (else
            (bind _returnvalue_6 (SaveGame|DoesSaveGameExist (Variables|Default|GetlevelsSaveSlot)))
            (if _returnvalue_6
              (bind _returnvalue_7 (SaveGame|LoadGamefromSlot _levelssaveslot_2))
              (bind _aspssave_game_2 (Utilities|Casting|CastToPSSaveGame _returnvalue_7))
              (Utilities|Array|Add (Variables|/Script/PrototypeStrategy.PSSaveGame|Getlevels _aspssave_game_2) (LocalVariables|GetLevelToSave))
              (SaveGame|SaveGametoSlot _returnvalue_7 _levelssaveslot_2)
              (else
                (bind _returnvalue_8 (SaveGame|CreateSaveGameObject "/Script/PrototypeStrategy.PSSaveGame"))
                (Utilities|Array|Add (Variables|/Script/PrototypeStrategy.PSSaveGame|Getlevels _returnvalue_8) (LocalVariables|GetLevelToSave))
                (SaveGame|SaveGametoSlot _returnvalue_8 _levelssaveslot_2)))))))))

(fn SaveLevels
  (params (Levels :type Array%20of%20Level%20Data%20Structures))
  (bind _levelssaveslot (Variables|Default|GetlevelsSaveSlot))
  (bind _returnvalue (SaveGame|DoesSaveGameExist (Variables|Default|GetlevelsSaveSlot)))
  (if _returnvalue
    (bind _returnvalue_2 (SaveGame|LoadGamefromSlot _levelssaveslot))
    (bind _aspssave_game (Utilities|Casting|CastToPSSaveGame _returnvalue_2))
    (Variables|/Script/PrototypeStrategy.PSSaveGame|Setlevels _aspssave_game Levels)
    (SaveGame|SaveGametoSlot _returnvalue_2 _levelssaveslot)
    (else
      (bind _returnvalue_3 (SaveGame|CreateSaveGameObject "/Script/PrototypeStrategy.PSSaveGame"))
      (Variables|/Script/PrototypeStrategy.PSSaveGame|Setlevels _returnvalue_3 Levels)
      (SaveGame|SaveGametoSlot _returnvalue_3 _levelssaveslot))))

(fn LoadSound
  (bind _returnvalue (SaveGame|DoesSaveGameExist "Volum"))
  (if _returnvalue
    (bind _returnvalue_2 (SaveGame|LoadGamefromSlot "Volum"))
    (bind _asbp_save_game (Utilities|Casting|CastToBP_SaveGame _returnvalue_2))
    (return (Variables|/Game/Project/GameMode/BP_SaveGame.BP_SaveGame_C|GetAllVolum _asbp_save_game) (Variables|/Game/Project/GameMode/BP_SaveGame.BP_SaveGame_C|GetEffectVolum _asbp_save_game) (Variables|/Game/Project/GameMode/BP_SaveGame.BP_SaveGame_C|GetMusicVolum _asbp_save_game))
    (else
      (bind _returnvalue_3 (SaveGame|CreateSaveGameObject "/Game/Project/GameMode/BP_SaveGame.BP_SaveGame_C"))
      (bind _output_get (Variables|Default|SetAs%20BP%20Save%20Game _returnvalue_3))
      (bind _output_get_2 (Variables|/Game/Project/GameMode/BP_SaveGame.BP_SaveGame_C|SetAllVolum _output_get 0.5))
      (bind _output_get_3 (Variables|/Game/Project/GameMode/BP_SaveGame.BP_SaveGame_C|SetEffectVolum _output_get 0.5))
      (bind _output_get_4 (Variables|/Game/Project/GameMode/BP_SaveGame.BP_SaveGame_C|SetMusicVolum _output_get 0.5))
      (SaveGame|SaveGametoSlot _output_get "Volum")
      (return _output_get_2 _output_get_3 _output_get_4))))

(fn SaveSound
  (params (All%20Volume :type Float%20%28single-precision%29) (Effects :type Float%20%28single-precision%29) (Music :type Float%20%28single-precision%29))
  (bind _returnvalue (SaveGame|LoadGamefromSlot "Volum"))
  (bind _asbp_save_game (Utilities|Casting|CastToBP_SaveGame _returnvalue))
  (Variables|/Game/Project/GameMode/BP_SaveGame.BP_SaveGame_C|SetAllVolum _asbp_save_game All%20Volume)
  (Variables|/Game/Project/GameMode/BP_SaveGame.BP_SaveGame_C|SetEffectVolum _asbp_save_game Effects)
  (Variables|/Game/Project/GameMode/BP_SaveGame.BP_SaveGame_C|SetMusicVolum _asbp_save_game Music)
  (SaveGame|SaveGametoSlot _asbp_save_game "Volum"))

(fn SaveInput
  (params (Restart :type Text) (Reset :type Input%20Key%20Selector%20Object%20Reference) (Reset1 :type Input%20Action%20Key%20Mapping%20Structure))
  (bind _returnvalue (SaveGame|LoadGamefromSlot "Input"))
  (bind _asbp_save_game (Utilities|Casting|CastToBP_SaveGame _returnvalue))
  (Variables|/Game/Project/GameMode/BP_SaveGame.BP_SaveGame_C|SetRestart _asbp_save_game Restart)
  (Variables|/Game/Project/GameMode/BP_SaveGame.BP_SaveGame_C|SetReset _asbp_save_game Reset1)
  (SaveGame|SaveGametoSlot _asbp_save_game "Input"))

(fn LoadInput
  (bind _returnvalue (SaveGame|DoesSaveGameExist "Input"))
  (if _returnvalue
    (bind _returnvalue_2 (SaveGame|LoadGamefromSlot "Input"))
    (bind _asbp_save_game (Utilities|Casting|CastToBP_SaveGame _returnvalue_2))
    (return (Variables|/Game/Project/GameMode/BP_SaveGame.BP_SaveGame_C|GetRestart _asbp_save_game) (Variables|/Game/Project/GameMode/BP_SaveGame.BP_SaveGame_C|GetReset _asbp_save_game))
    (else
      (bind _returnvalue_3 (SaveGame|CreateSaveGameObject "/Game/Project/GameMode/BP_SaveGame.BP_SaveGame_C"))
      (bind _output_get (Variables|Default|SetAs%20BP%20Save%20Game _returnvalue_3))
      (bind _output_get_2 (Variables|/Game/Project/GameMode/BP_SaveGame.BP_SaveGame_C|SetRestart _output_get (Variables|/Game/Project/GameMode/BP_SaveGame.BP_SaveGame_C|GetRestart _asbp_save_game)))
      (bind _output_get_3 (Variables|/Game/Project/GameMode/BP_SaveGame.BP_SaveGame_C|SetReset _output_get ""))
      (SaveGame|SaveGametoSlot _output_get "Input")
      (return _output_get_2 _output_get_3))))