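; BP_Mine_Menu_GM is the menu game mode.
; On BeginPlay it sets the base sound mix, caches the game instance and, if the levels save slot exists, loads the level-unlock save.
; It only prints each saved level to screen, without applying the data.
; Disconnected leftover graphs for switching music tracks, a sound pack and menu music never run.
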(event EventBeginPlay
  (Class|GameplayStatics|SetBaseSoundMix "/Game/Project/Sound/SM_SoundGame.SM_SoundGame")
  (bind _asbp_main_game_instance (Utilities|Casting|CastToBP_MainGameInstance (Game|GetGameInstance)))
  (bind _output_get (Variables|Default|SetAs%20BP%20Main%20Game%20Instance _asbp_main_game_instance))
  (bind _returnvalue (SaveGame|DoesSaveGameExist (Variables|/Script/PrototypeStrategy.PSGameInstance|GetlevelsSaveSlot _output_get)))
  (if _returnvalue
    (bind _returnvalue_2 (SaveGame|LoadGamefromSlot (Variables|/Script/PrototypeStrategy.PSGameInstance|GetlevelsSaveSlot _output_get)))
    (bind _asbp_save_level_unlock (Utilities|Casting|CastToBP_SaveLevelUnlock _returnvalue_2))
    (for _array_element (Variables|/Game/Project/Core/Save/BP_SaveLevelUnlock.BP_SaveLevelUnlock_C|GetLevels _asbp_save_level_unlock)
      (Development|PrintString (Utilities|String|ToString(Integer) (.Level (Utilities|Struct|BreakS_SaveLevels _array_element)))))))

(fn ConstructionScript)