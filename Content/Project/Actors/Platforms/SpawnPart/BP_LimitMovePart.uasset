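; Platform part Blueprint that changes its look as a move limit changes, through the CheckandChangeColorCode event.
; The event divides current limit by starting limit and looks up that ratio in the ColorMaterials map to set the flipbook, or else the sprite.
; A failed lookup loops over the keys, though its same-bound clamp only matches exact values.
; Older tint and material-parameter logic remains disconnected.
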(event EventBeginPlay)

(event EventCheckandChangeColorCode
  (params (limitOnStart :type Integer) (currentLimit :type Integer))
  (bind _returnvalue (Math|Conversions|ToFloat(Integer) currentLimit))
  (bind _returnvalue_2 (Math|Conversions|ToFloat(Integer) limitOnStart))
  (bind _sprite (Variables|Default|GetSprite))
  (bind _flipbook (Variables|Default|GetFlipbook))
  (bind _colormaterials (Variables|Default|GetColorMaterials))
  (bind _materials (Utilities|Struct|BreakColorsType _colormaterials))
  (bind _returnvalue_3 (Class|PaperFlipbookComponent|GetFlipbook _flipbook))
  (bind _returnvalue_4 (Sprite|GetSprite _sprite))
  (bind _returnvalue_5 (/ _returnvalue _returnvalue_2))
  (bind (_value _returnvalue_6) (Utilities|Map|Find _materials _returnvalue_5))
  (bind (_flipbookmaterial _spritematerial) (Utilities|Struct|BreakMaterialsType _value))
  ;[1 1 1] Comment
  (if _returnvalue_6
    (Utilities|IsValid (Variables|Default|GetFlipbook)
      (:Is%20Valid
        (Sprite|SetFlipbook (Variables|Default|GetFlipbook) _flipbookmaterial))
      (:Is%20Not%20Valid
        (Utilities|IsValid (Variables|Default|GetSprite)
          (:Is%20Valid
            (Rendering|Components|Sprite|SetSprite (Variables|Default|GetSprite) _spritematerial)))))
    (else
      (bind _keys (Utilities|Map|Keys _materials))
      (bind _array_element (Utilities|Array|ForEachLoopwithBreak _keys :!label _label)
        (:LoopBody
          (if (== _array_element 1.0)
            (Variables|Default|SetArray%20Element _array_element)
            (elif (== _returnvalue_5 (Math|Float|Clamp(Float) _returnvalue_5 _array_element (Variables|Default|GetArray%20Element)))
              (if (.ReturnValue (Utilities|Map|Find (Utilities|Struct|BreakColorsType (Variables|Default|GetColorMaterials)) (Variables|Default|GetArray%20Element)))
                (Utilities|IsValid _returnvalue_3
                  (:Is%20Valid
                    (if (== (.FlipbookMaterial (Utilities|Struct|BreakMaterialsType (.Value (Utilities|Map|Find (Utilities|Struct|BreakColorsType (Variables|Default|GetColorMaterials)) (Variables|Default|GetArray%20Element))))) _returnvalue_3)
                      (goto _label Break)
                      (else
                        (Sprite|SetFlipbook (Variables|Default|GetFlipbook) (.FlipbookMaterial (Utilities|Struct|BreakMaterialsType (.Value (Utilities|Map|Find (Utilities|Struct|BreakColorsType (Variables|Default|GetColorMaterials)) (Variables|Default|GetArray%20Element))))))
                        (goto _label Break))))
                  (:Is%20Not%20Valid
                    (Utilities|IsValid _returnvalue_4
                      (:Is%20Valid
                        (if (== (.SpriteMaterial (Utilities|Struct|BreakMaterialsType (.Value (Utilities|Map|Find (Utilities|Struct|BreakColorsType (Variables|Default|GetColorMaterials)) (Variables|Default|GetArray%20Element))))) _returnvalue_4)
                          (Rendering|Components|Sprite|SetSprite (Variables|Default|GetSprite) (.SpriteMaterial (Utilities|Struct|BreakMaterialsType (.Value (Utilities|Map|Find (Utilities|Struct|BreakColorsType (Variables|Default|GetColorMaterials)) (Variables|Default|GetArray%20Element))))))
                          (goto _label Break)))))))
              (else
                (Variables|Default|SetArray%20Element _array_element)))))))))

(fn ConstructionScript)