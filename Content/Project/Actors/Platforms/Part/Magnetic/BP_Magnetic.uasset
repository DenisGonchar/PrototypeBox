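; BP_Magnetic is a magnetic platform part with a clickable polarization state.
; Clicking its box component cycles Polarization through None, Positive and Negative and prints the new value.
; A separate ChangeMaterial_1 event swaps the mesh between two materials from a boolean, independent of polarization.
; No magnetic force is applied here, and a forward line trace sits unconnected, so it never runs.
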(event OnClicked(BoxComponent)
  (params (TouchedComponent :type Primitive%20Component%20Object%20Reference) (ButtonPressed :type Key%20Structure :default "None"))
  (switch Utilities|FlowControl|Switch|SwitchonEPolarizationType (Variables|Default|Getpolarization)
    (:None
      (Variables|Default|Setpolarization "Positive"))
    (:Positive
      (Variables|Default|Setpolarization "Negative"))
    (:Negative
      (Variables|Default|Setpolarization "None")))
  (Development|PrintString (Utilities|String|EnumtoString (Variables|Default|Getpolarization))))

(event Custom|ChangeMaterial_1
  (params (value :type Boolean))
  (bind _staticmesh1 (Variables|Default|GetStaticMesh1))
  (if value
    (Rendering|Material|SetMaterial _staticmesh1 0 "/Engine/MapTemplates/Materials/BasicAsset03.BasicAsset03")
    (else
      (Rendering|Material|SetMaterial _staticmesh1 0 "/Engine/MapTemplates/Materials/BasicAsset01.BasicAsset01"))))

(event EventBeginPlay)

(event Collision|EventActorBeginOverlap
  (params (OtherActor :type Actor%20Object%20Reference)))

(event EventTick
  (params (DeltaSeconds :type Float%20%28single-precision%29)))

(fn ConstructionScript)