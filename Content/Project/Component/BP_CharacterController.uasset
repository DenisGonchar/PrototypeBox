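; Player controller that sets up the game HUD and routes pause and mouse-click input.
; On BeginPlay, outside the "Constructor" level, it adds the BPW_Game widget to the viewport and caches the main game instance.
; The 0 and Escape keys ask that game instance to show the pause menu.
; Mouse clicks trace under the cursor on the Visibility channel and pass the result to CallMouseClicked.
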(event EventBeginPlay
  (bind _returnvalue (Game|GetCurrentLevelName true))
  (if (Utilities|Enum|NotEqual(Enum) _returnvalue "Constructor")
    (bind _returnvalue_2 (UserInterface|CreateWidget "/Game/Project/Widget/BP/BPW_Game.BPW_Game_C"))
    (bind _output_get (Variables|Default|SetGameWidget _returnvalue_2))
    (UserInterface|Viewport|AddtoViewport _output_get 0)
    (bind _asbp_main_game_instance (Utilities|Casting|CastToBP_MainGameInstance (Game|GetGameInstance)))
    (Variables|Default|SetAs%20BP%20Main%20Game%20Instance _asbp_main_game_instance)))

(event EventTick
  (params (DeltaSeconds :type Float%20%28single-precision%29)))

(event Input|ActionEvents|InputActionMouseClicked
  (params (Key :type Key%20Structure :default "None"))
  (bind (_hitresult _returnvalue) (Game|Player|GetHitResultUnderCursorbyChannel "TraceTypeQuery1" false))
  (:Pressed
    (Default|CallMouseClicked _hitresult _returnvalue)))

(event Input|KeyboardEvents|Escape
  (params (Key :type Key%20Structure :default "None"))
  (:Pressed
    (Default|ShowPauseMenu (Variables|Default|GetAs%20BP%20Main%20Game%20Instance))))

(event Input|KeyboardEvents|0
  (params (Key :type Key%20Structure :default "None"))
  (:Pressed
    (Default|ShowPauseMenu (Variables|Default|GetAs%20BP%20Main%20Game%20Instance))))

(fn ConstructionScript)